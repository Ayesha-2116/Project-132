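; Player controller component that runs the in-game text chat, linking each player's chat widget to the other players.
; On BeginPlay, the local controller creates the chat UI and caches its chatbox, which Enter focuses and the mouse wheel scrolls.
; A server-named send event loops through the GameState PlayerArray and calls each controller component's owning-client event, which adds the message to that player's chatbox.
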(event `self.ReceiveBeginPlay`
  (if (`Controller.IsLocalPlayerController` (cast `PlayerController` (`self.GetOwner`) :!pure true))
    (bind _returnvalue (`|CreateWidget` "/Game/Chat/WB_ChatUI.WB_ChatUI_C"))
    (bind _output_get (set `self.ChatUI_Ref` _returnvalue))
    (`UserWidget.AddToViewport` _output_get 0)
    (set `self.Chatbox_Ref` (`/Game/Chat/WB_ChatUI.WB_Chatbox` _output_get))))

(event `Key|Enter`
  (params (Key :type "Key Structure"))
  (:`Pressed`
    (`/Game/Chat/WB_Chatbox.FocusChat` (`self.Chatbox_Ref`))))

(event `Key|MouseScrollUp`
  (params (Key :type "Key Structure"))
  (:`Pressed`
    (`/Game/Chat/WB_Chatbox.Scroll` (`self.Chatbox_Ref`) true)))

(event `Key|MouseScrollDown`
  (params (Key :type "Key Structure"))
  (:`Pressed`
    (`/Game/Chat/WB_Chatbox.Scroll` (`self.Chatbox_Ref`) false)))

(event `SendChatMessageOnServer`
  (params (Message :type String))
  (for _array_element (`GameStateBase.PlayerArray` (`GameplayStatics.GetGameState`))
    (`self.AddChatMEssagesOnOWningClient` (`Actor.GetComponentByClass` (`PlayerState.GetPlayerController` _array_element) "AC_Chat_PC_C") Message)))

(event `AddChatMEssagesOnOWningClient`
  (params (Message :type String))
  (`/Game/Chat/WB_Chatbox.AddChatMessage` (`self.Chatbox_Ref`) Message))